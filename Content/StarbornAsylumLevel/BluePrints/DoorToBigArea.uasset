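; DoorToBigArea is a sliding door that opens on E once the game mode's CollectablesLeft count reaches zero.
; A Box overlap with the first-person character enables or disables the door's input, limiting the key to nearby players.
; The DoorSlide timeline moves the StaticMesh while a sound plays at the door.
; A Delay chained from the timeline's Update reverses the slide a few seconds later.
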(event `Key|E`
  (params (Key :type "Key Structure"))
  (:`Pressed`
    (bind _asbp_first_person_game_mode (cast `/Game/FirstPerson/Blueprints/BP_FirstPersonGameMode` (`GameplayStatics.GetGameMode`)))
    (if (== (`/Game/FirstPerson/Blueprints/BP_FirstPersonGameMode.Collectables Left` _asbp_first_person_game_mode) 0)
      (`|ExecutionSequence`
        (:`then_0`
          (bind (_direction _slide2) (`Timeline|DoorSlide` :`NewTime` 0.0 :!label _label)
            (:`Update`
              (`SceneComponent.K2_SetRelativeLocation` (`self.StaticMesh`) _slide2 false false)
              (`KismetSystemLibrary.Delay` 4.0)
              (goto _label :!via `Reverse`))))
        (:`then_1`
          (`GameplayStatics.PlaySoundAtLocation` "/Game/Sound/Cues/dooropen_cue.dooropen_cue" (`self.K2_GetActorLocation`) (struct) 1.0 1.0 0.0 null null null null))))))

(event `self.Box.OnComponentBeginOverlap`
  (params (OverlappedComponent :type "PrimitiveComponent Object Reference") (OtherActor :type "Actor Object Reference") (OtherComp :type "PrimitiveComponent Object Reference") (OtherBodyIndex :type Integer) (bFromSweep :type Boolean) (SweepResult :type "HitResult Structure (by ref)"))
  (cast `/Game/FirstPerson/Blueprints/BP_FirstPersonCharacter` OtherActor)
  (`self.EnableInput` (`GameplayStatics.GetPlayerController` 0)))

(event `self.Box.OnComponentEndOverlap`
  (params (OverlappedComponent :type "PrimitiveComponent Object Reference") (OtherActor :type "Actor Object Reference") (OtherComp :type "PrimitiveComponent Object Reference") (OtherBodyIndex :type Integer))
  (cast `/Game/FirstPerson/Blueprints/BP_FirstPersonCharacter` OtherActor)
  (`self.DisableInput` (`GameplayStatics.GetPlayerController` 0)))

(fn `UserConstructionScript`)