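; Interactable button in the Starborn Asylum level that lifts the lockdown and opens the doors linked to it.
; A box overlap shows or hides its prompt for the first-person character.
; Interact opens the first InteractDoorBP whose value matches ButtonValue and switches the player's view to it.
; It also hides the prompt, plays an alarm, sets LockdownLifted on the game mode and opens all matching DownstairsPatient doors.
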(event `/Game/StarbornAsylumLevel/BluePrints/InteractInterface.Interact`
  (params (Player :type "/Game/FirstPerson/Blueprints/BP_FirstPersonCharacter Object Reference"))
  (`|ExecutionSequence`
    (:`then_0`
      (bind _outactors (`GameplayStatics.GetAllActorsOfClass` "/Game/StarbornAsylumLevel/BluePrints/InteractDoorBP.InteractDoorBP_C"))
      (for _array_element _outactors
        (if (== (`/Game/StarbornAsylumLevel/BluePrints/InteractDoorBP.DoorValue` _array_element) (`self.ButtonValue`))
          (`/Game/StarbornAsylumLevel/BluePrints/InteractDoorBP.OpenDoor` _array_element Player)
          (`PlayerController.SetViewTargetWithBlend` (`GameplayStatics.GetPlayerController` 0) _array_element 0.0 "VTBlend_Linear" 0.0 false)
          (break))))
    (:`then_1`
      (`SceneComponent.SetHiddenInGame` (`self.Prompt`) true false))
    (:`then_2`
      (`GameplayStatics.PlaySound2D` "/Game/Sound/alarm2.alarm2" 1.0 1.0 0.0 null null))
    (:`then_3`
      (bind _asbp_first_person_game_mode (cast `/Game/FirstPerson/Blueprints/BP_FirstPersonGameMode` (`GameplayStatics.GetGameMode`)))
      (set `/Game/FirstPerson/Blueprints/BP_FirstPersonGameMode.LockdownLifted?` true _asbp_first_person_game_mode))
    (:`then_4`
      (bind _outactors_2 (`GameplayStatics.GetAllActorsOfClass` "/Game/StarbornAsylumLevel/BluePrints/DownstairsPatient.DownstairsPatient_C"))
      (for _array_element_2 _outactors_2
        (if (== (`/Game/StarbornAsylumLevel/BluePrints/DownstairsPatient.PatientDoorValue` _array_element_2) (`self.ButtonValue`))
          (`/Game/StarbornAsylumLevel/BluePrints/DownstairsPatient.Open Door` _array_element_2))))))

(event `self.Box.OnComponentBeginOverlap`
  (params (OverlappedComponent :type "PrimitiveComponent Object Reference") (OtherActor :type "Actor Object Reference") (OtherComp :type "PrimitiveComponent Object Reference") (OtherBodyIndex :type Integer) (bFromSweep :type Boolean) (SweepResult :type "HitResult Structure (by ref)"))
  (cast `/Game/FirstPerson/Blueprints/BP_FirstPersonCharacter` OtherActor)
  (`SceneComponent.SetHiddenInGame` (`self.Prompt`) false false))

(event `self.Box.OnComponentEndOverlap`
  (params (OverlappedComponent :type "PrimitiveComponent Object Reference") (OtherActor :type "Actor Object Reference") (OtherComp :type "PrimitiveComponent Object Reference") (OtherBodyIndex :type Integer))
  (cast `/Game/FirstPerson/Blueprints/BP_FirstPersonCharacter` OtherActor)
  (`SceneComponent.SetHiddenInGame` (`self.Prompt`) true false))

(fn `UserConstructionScript`)