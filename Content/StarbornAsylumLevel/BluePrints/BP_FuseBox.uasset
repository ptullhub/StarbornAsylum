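; BP_FuseBox is an interactable fuse box that the player can activate once, as long as they are not carrying the gun.
; Overlapping its Box with the first-person character shows a Widget prompt and enables input, and leaving reverses both.
; Pressing Interact calls ActivateFuseBox on BP_FirstPersonGameMode and plays a shock sound.
; It then disables input, hides the prompt and destroys the trigger and Sparks components, preventing reuse.
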(event `InputAction|Interact`
  (params (Key :type "Key Structure"))
  (:`Pressed`
    (bind _returnvalue (`GameplayStatics.GetActorOfClass` "/Game/FirstPerson/Blueprints/BP_FirstPersonGameMode.BP_FirstPersonGameMode_C"))
    (if (not (`/Game/FirstPerson/Blueprints/BP_FirstPersonCharacter.HasGun?` (stale `self.Box.OnComponentBeginOverlap` _asbp_first_person_character)))
      (`/Game/FirstPerson/Blueprints/BP_FirstPersonGameMode.ActivateFuseBox` _returnvalue)
      (`GameplayStatics.PlaySound2D` "/Game/Sound/shocksound.shocksound" 1.0 1.0 0.0 null null)
      (`self.DisableInput` null)
      (`SceneComponent.SetHiddenInGame` (`self.Widget`) true false)
      (`ActorComponent.K2_DestroyComponent` (`self.Box`))
      (`ActorComponent.K2_DestroyComponent` (`self.Sparks`)))))

(event `self.Box.OnComponentBeginOverlap`
  (params (OverlappedComponent :type "PrimitiveComponent Object Reference") (OtherActor :type "Actor Object Reference") (OtherComp :type "PrimitiveComponent Object Reference") (OtherBodyIndex :type Integer) (bFromSweep :type Boolean) (SweepResult :type "HitResult Structure (by ref)"))
  (bind _asbp_first_person_character (cast `/Game/FirstPerson/Blueprints/BP_FirstPersonCharacter` OtherActor))
  (`SceneComponent.SetHiddenInGame` (`self.Widget`) false false)
  (`self.EnableInput` (`GameplayStatics.GetPlayerController` 0)))

(event `self.Box.OnComponentEndOverlap`
  (params (OverlappedComponent :type "PrimitiveComponent Object Reference") (OtherActor :type "Actor Object Reference") (OtherComp :type "PrimitiveComponent Object Reference") (OtherBodyIndex :type Integer))
  (cast `/Game/FirstPerson/Blueprints/BP_FirstPersonCharacter` OtherActor)
  (`SceneComponent.SetHiddenInGame` (`self.Widget`) true false)
  (`self.DisableInput` null))

(fn `UserConstructionScript`)