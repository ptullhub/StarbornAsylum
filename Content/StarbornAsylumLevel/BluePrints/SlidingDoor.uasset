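; Sliding door Blueprint in the Starborn Asylum level that opens when something overlaps its Box and closes when the overlap ends.
; The DoorSlide timeline plays forward or reverses to set the static mesh's relative location.
; A DoOnce, re-armed when the timeline finishes, gates the opening sound, while the closing sound plays after a short delay.
; Overlaps are not filtered by actor type.
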(event `self.Box.OnComponentBeginOverlap`
  (params (OverlappedComponent :type "PrimitiveComponent Object Reference") (OtherActor :type "Actor Object Reference") (OtherComp :type "PrimitiveComponent Object Reference") (OtherBodyIndex :type Integer) (bFromSweep :type Boolean) (SweepResult :type "HitResult Structure (by ref)"))
  (`|ExecutionSequence`
    (:`then_0`
      (bind (_direction _doorslide) (`Timeline|DoorSlide` :!label _label)
        (:`Update`
          (`SceneComponent.K2_SetRelativeLocation` (`self.StaticMesh`) _doorslide false false))
        (:`Finished`
          (goto _label_2 :!via `Reset`))))
    (:`then_1`
      (`/Engine/EditorBlueprintResources/StandardMacros.DoOnce` false :!label _label_2
        (:`Completed`
          (`GameplayStatics.PlaySoundAtLocation` "/Game/Sound/Cues/dooropen_cue.dooropen_cue" (`self.K2_GetActorLocation`) (struct) 1.0 1.0 0.0 null null null null))))))

(event `self.Box.OnComponentEndOverlap`
  (params (OverlappedComponent :type "PrimitiveComponent Object Reference") (OtherActor :type "Actor Object Reference") (OtherComp :type "PrimitiveComponent Object Reference") (OtherBodyIndex :type Integer))
  (`|ExecutionSequence`
    (:`then_0`
      (`KismetSystemLibrary.Delay` 1.5)
      (`GameplayStatics.PlaySoundAtLocation` "/Game/Sound/Cues/doorclosed_cue.doorclosed_cue" (`self.K2_GetActorLocation`) (struct) 1.0 1.0 0.0 null null null null))
    (:`then_1`
      (goto _label :!via `Reverse`))))

(fn `UserConstructionScript`)