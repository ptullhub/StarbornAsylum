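; Test zombie AI pawn that roams the level, chases pawns it sees and dies when its health runs out.
; It loops AI MoveTo to random reachable points around itself, pausing briefly between moves.
; Pawn Sensing sightings start a move toward the seen pawn, and a retriggerable delay resumes roaming once sightings stop.
; Any damage lowers health, refreshes the health bar widget linked at BeginPlay, and destroys the actor at zero.
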(event `self.ReceiveAnyDamage`
  (params (Damage :type "Float (single-precision)") (DamageType :type "DamageType Object Reference") (InstigatedBy :type "Controller Object Reference") (DamageCauser :type "Actor Object Reference"))
  ;[1 1 1] Checks and updates health and then destroys the actor if they reach 0 health or less (Reminder, healthbar can be hidden by clicking on it in the hierarchy and enabling "Hidden in Game)
  (bind _output_get (set `self.Health` (- (`self.Health`) Damage)))
  (`/Game/Widgets/EnemyHealth.UpdateHealth` (`self.EnemyHealthBarWidget`))
  (if (<= _output_get 0.0)
    (`self.K2_DestroyActor`)))

(event `self.ReceiveBeginPlay`
  ;[1 1 1] Roaming
  (`|ExecutionSequence`
    (:`then_0`
      ;[1 1 1] Checks and updates health and then destroys the actor if they reach 0 health or less (Reminder, healthbar can be hidden by clicking on it in the hierarchy and enabling "Hidden in Game)
      (bind _asenemy_health (cast `/Game/Widgets/EnemyHealth` (`WidgetComponent.GetUserWidgetObject` (`self.EnemyHealthBar`))))
      (bind _output_get (set `self.EnemyHealthBarWidget` _asenemy_health))
      (set `/Game/Widgets/EnemyHealth.Enemy` self _output_get)
      (`/Game/Widgets/EnemyHealth.UpdateHealth` _output_get))
    (:`then_1`
      (`self.Random Roam`))))

(event `Random Roam`
  ;[1 1 1] Roaming
  (`|AIMoveTo` self (`NavigationSystemV1.K2_GetRandomReachablePointInRadius` (`self.K2_GetActorLocation`) 2500.0 null null) null
    (:`OnSuccess`
      (`KismetSystemLibrary.Delay` 1.0)
      (`self.Random Roam`))))

(event `self.PawnSensing.OnSeePawn`
  (params (Pawn :type "Pawn Object Reference"))
  ;[1 1 1] Player Sighted
  (`|ExecutionSequence`
    (:`then_0`
      (`|AIMoveTo` self (0.0 0.0 0.0) Pawn))
    (:`then_1`
      (`KismetSystemLibrary.RetriggerableDelay` 2.0)
      (`self.Random Roam`))))

(fn `UserConstructionScript`)