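; BP_AIZombie is a test zombie AI pawn that roams the level and chases pawns it sees.
; On BeginPlay it moves to random reachable points around itself, pausing briefly after each successful move before picking the next.
; When PawnSensing sees a pawn it moves toward that actor, and a retriggerable delay restarts roaming shortly after sightings stop.
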(event `self.ReceiveBeginPlay`
  ;[1 1 1] Roaming
  (`self.Random Roam`))

(event `Random Roam`
  ;[1 1 1] Roaming
  (`|AIMoveTo` self (`NavigationSystemV1.K2_GetRandomReachablePointInRadius` (`self.K2_GetActorLocation`) 2500.0 null null) null
    (:`OnSuccess`
      (`KismetSystemLibrary.Delay` 3.0)
      (`self.Random Roam`))))

(event `self.PawnSensing.OnSeePawn`
  (params (Pawn :type "Pawn Object Reference"))
  ;[1 1 1] Player Sighted
  (`|ExecutionSequence`
    (:`then_0`
      (`|AIMoveTo` self (0.0 0.0 0.0) Pawn))
    (:`then_1`
      (`KismetSystemLibrary.RetriggerableDelay` 2.0)
      (`self.Random Roam`))))

(fn `UserConstructionScript`)