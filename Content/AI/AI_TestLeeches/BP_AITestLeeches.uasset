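; BP_AITestLeeches is a test AI gunman with a revolver, health and a death sequence.
; BeginPlay caches the mesh's LeechesAnimation instance.
; FireRevoler attaches a muzzle effect to the revolver and spawns BP_LeechesProjectile at ProjectileSpawn, but nothing in this graph calls it.
; AnyDamage lowers Health; at zero or below it plays a kneel animation, removes the revolver and destroys the actor after a short gameplay-task delay.
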(event `self.ReceiveBeginPlay`
  (`|ExecutionSequence`
    (:`then_1`
      (bind _asleeches_animation (cast `/Game/AI/AI_TestLeeches/LeechesAnimation` (`SkeletalMeshComponent.GetAnimInstance` (`self.Mesh`))))
      (set `self.AnimInstance` _asleeches_animation))))

(event `self.ReceiveAnyDamage`
  (params (Damage :type "Float (single-precision)") (DamageType :type "DamageType Object Reference") (InstigatedBy :type "Controller Object Reference") (DamageCauser :type "Actor Object Reference"))
  ;[1 1 1] Checks and updates health and then destroys the actor if they reach 0 health or less
  (set `self.Health` (- (`self.Health`) Damage))
  (if (<= (`self.Health`) 0.0)
    (`SkeletalMeshComponent.PlayAnimation` (`self.Mesh`) "/Game/AI/AI_TestLeeches/Animations/unused/pistol_stand_to_kneel.pistol_stand_to_kneel" false)
    (`ActorComponent.K2_DestroyComponent` (`self.Revolver`))
    (bind _returnvalue (`AddComponent|NODE_AddGameplayTasksComponent-0`))
    (`GameplayTask_WaitDelay.TaskWaitDelay` _returnvalue 1.0
      (:`OnFinish`
        (`self.K2_DestroyActor`)))))

(event `FireRevoler`
  (bind _projectilespawn (`self.ProjectileSpawn`))
  (`GameplayStatics.SpawnEmitterAttached` "/Game/FXVarietyPack/Particles/P_ky_explosion2.P_ky_explosion2" (`self.Revolver`) "None" (-0.366874 13.0 14.372444) (struct) (0.05 0.05 0.05))
  (`|SpawnActorFromClass` "/Game/AI/AI_TestLeeches/Revolver/Projectile/BP_LeechesProjectile.BP_LeechesProjectile_C" (`KismetMathLibrary.MakeTransform` (`SceneComponent.K2_GetComponentLocation` _projectilespawn) (`SceneComponent.K2_GetComponentRotation` _projectilespawn)) "Undefined" "OverrideRootScale" null null))

(fn `UserConstructionScript`)