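; BP_ZombieChar is the zombie enemy character that melee-attacks the first-person player and handles its own death.
; AttackPlayer plays the attack montage, waits for a delay, then damages the player only if still within melee range.
; AnyDamage subtracts from Health; at zero it plays the dying animation, notifies BP_ZombieController via Killed, and destroys the actor after a delay.
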(event `AttackPlayer`
  ;[1 1 1] Plays the attack animation and applies damage if in melee range
  (`|PlayMontage` (`self.Mesh`) "/Game/AI/AI_Zombie/Animations/Zombie1_Attack_Montage.Zombie1_Attack_Montage"
    (:`then`
      (bind _asbp_first_person_character (cast `/Game/FirstPerson/Blueprints/BP_FirstPersonCharacter` (`GameplayStatics.GetPlayerCharacter` 0)))
      (`KismetSystemLibrary.Delay` 1.2)
      (if (<= (`self.GetDistanceTo` _asbp_first_person_character) 200.0)
        (`GameplayStatics.ApplyDamage` _asbp_first_person_character 2.0)))))

(event `self.ReceiveAnyDamage`
  (params (Damage :type "Float (single-precision)") (DamageType :type "DamageType Object Reference") (InstigatedBy :type "Controller Object Reference") (DamageCauser :type "Actor Object Reference"))
  ;[1 1 1] Handles AI Death
  (set `self.Health` (- (`self.Health`) Damage))
  (if (<= (`self.Health`) 0.0)
    (`SkeletalMeshComponent.PlayAnimation` (`self.Mesh`) "/Game/AI/AI_Zombie/Animations/Zombie1_Dying_Anim_mixamo_com.Zombie1_Dying_Anim_mixamo_com" false)
    (bind _asbp_zombie_controller (cast `/Game/AI/AI_Zombie/Logic/BP_ZombieController` (`self.GetController`)))
    (`/Game/AI/AI_Zombie/Logic/BP_ZombieController.Killed` _asbp_zombie_controller)
    (`KismetSystemLibrary.Delay` 5.0)
    (`self.K2_DestroyActor`)))

(fn `UserConstructionScript`)