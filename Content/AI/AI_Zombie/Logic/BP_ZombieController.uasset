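; BP_ZombieController is the AI controller for zombie pawns, running the BT_Zombie behavior tree when play begins.
; Its perception update casts the sensed actor to the first-person player character and writes the sensing result to the HasSpottedPlayer blackboard key, so spotting and losing the player both update it.
; A Killed event detaches the controller from the pawn through DetachFromControllerPendingDestroy.
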(event `Killed`
  (`Pawn.DetachFromControllerPendingDestroy` (`self.K2_GetPawn`)))

(event `self.ReceiveBeginPlay`
  (`self.RunBehaviorTree` "/Game/AI/AI_Zombie/Logic/BT_Zombie.BT_Zombie"))

(event `self.AIPerception.OnTargetPerceptionUpdated`
  (params (Actor :type "Actor Object Reference") (Stimulus :type "AIStimulus Structure"))
  (set `self.HasSensed` (`.bSuccessfullySensed` (break `AIStimulus` Stimulus)))
  (cast `/Game/FirstPerson/Blueprints/BP_FirstPersonCharacter` Actor)
  (`BlackboardComponent.SetValueAsBool` (`AIBlueprintHelperLibrary.GetBlackboard` null) "HasSpottedPlayer" (`self.HasSensed`)))

(fn `UserConstructionScript`)