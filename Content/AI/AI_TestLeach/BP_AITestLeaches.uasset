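; BP_AITestLeaches is a test Leach AI actor that takes damage and has a revolver firing effect.
; On BeginPlay it caches its mesh's anim instance as LeachesAnimation.
; Incoming damage is subtracted from Health, and the actor is destroyed once Health reaches zero or below.
; The FireRevoler event only spawns an explosion particle attached to the Revolver component, with no shot or damage logic.
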(event `self.ReceiveBeginPlay`
  (`|ExecutionSequence`
    (:`then_1`
      (bind _asleaches_animation (cast `/Game/AI/AI_TestLeach/LeachesAnimation` (`SkeletalMeshComponent.GetAnimInstance` (`self.Mesh`))))
      (set `self.AnimInstance` _asleaches_animation))))

(event `self.ReceiveAnyDamage`
  (params (Damage :type "Float (single-precision)") (DamageType :type "DamageType Object Reference") (InstigatedBy :type "Controller Object Reference") (DamageCauser :type "Actor Object Reference"))
  ;[1 1 1] Checks and updates health and then destroys the actor if they reach 0 health or less
  (set `self.Health` (- (`self.Health`) Damage))
  (if (<= (`self.Health`) 0.0)
    (`self.K2_DestroyActor`)))

(event `FireRevoler`
  (`GameplayStatics.SpawnEmitterAttached` "/Game/FXVarietyPack/Particles/P_ky_explosion2.P_ky_explosion2" (`self.Revolver`) "None" (-0.366874 13.0 14.372444) (struct) (0.05 0.05 0.05)))

(fn `UserConstructionScript`)